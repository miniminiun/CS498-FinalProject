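; BP_fireball is a fireball hazard, filed under FinalEnemy, that damages the player on contact.
; Tick moves it along the world Z axis at a rate driven by Speed, scaled by delta time.
; Its Sphere overlap destroys it one second after touching an actor tagged "land"; otherwise it reduces an overlapping PlayerCharacter's health through UpdateHealth without destroying itself.
; A lifespan set on BeginPlay also limits how long it exists.
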(event `self.ReceiveBeginPlay`
  (`self.SetLifeSpan` 10.0))

(event `self.ReceiveTick`
  (params (DeltaSeconds :type "Float (single-precision)"))
  (bind _result (`/Engine/EditorBlueprintResources/StandardMacros.NegateFloat` (* DeltaSeconds (`self.speed`)))
    (:`  `
      (`self.K2_AddActorWorldOffset` (`KismetMathLibrary.MakeVector` 0.0 0.0 _result)))))

(event `self.Sphere.OnComponentBeginOverlap`
  (params (OverlappedComponent :type "PrimitiveComponent Object Reference") (OtherActor :type "Actor Object Reference") (OtherComp :type "PrimitiveComponent Object Reference") (OtherBodyIndex :type Integer) (bFromSweep :type Boolean) (SweepResult :type "HitResult Structure (by ref)"))
  (if (`self.ActorHasTag` OtherActor "land")
    (`KismetSystemLibrary.Delay` 1.0)
    (`self.K2_DestroyActor`)
    (else
      (bind _asplayer_character (cast `/Game/PlayerDesign/Blueprints/PlayerCharacter` OtherActor))
      (`/Game/PlayerDesign/Blueprints/PlayerCharacter.UpdateHealth` _asplayer_character -10.0))))

(fn `UserConstructionScript`)