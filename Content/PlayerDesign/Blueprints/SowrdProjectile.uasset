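; Sword projectile actor that travels along its Velocity and damages the first enemy it overlaps.
; Tick counts down TimeRemains, moving the actor with a swept, scaled offset until the timer expires and destroys it.
; Mesh overlap deals a fraction of the PlayerCharacter's ATK to EnemyParent_BP through UpdateHPIgnoreCD, ignoring the player and non-enemies.
; After a hit the mesh is hidden and its collision disabled, leaving destruction to the timer.
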(event `self.ReceiveTick`
  (params (DeltaSeconds :type "Float (single-precision)"))
  (bind _output_get (set `self.Time Remains` (- (`self.Time Remains`) DeltaSeconds)))
  (if (<= _output_get 0.0)
    (`self.K2_DestroyActor`)
    (else
      (`self.K2_AddActorWorldOffset` (* (* (`self.velocity`) DeltaSeconds) 600.0) true))))

(event `self.StaticMesh.OnComponentBeginOverlap`
  (params (OverlappedComponent :type "PrimitiveComponent Object Reference") (OtherActor :type "Actor Object Reference") (OtherComp :type "PrimitiveComponent Object Reference") (OtherBodyIndex :type Integer) (bFromSweep :type Boolean) (SweepResult :type "HitResult Structure (by ref)"))
  (bind _staticmesh (`self.StaticMesh`))
  (cast `/Game/PlayerDesign/Blueprints/PlayerCharacter` OtherActor
    (:`CastFailed`
      (bind _asenemy_parent_bp (cast `/Game/ThirdPersonBP/Blueprints2/EnemyParent_BP` OtherActor))
      (bind _returnvalue (`GameplayStatics.GetActorOfClass` "/Game/PlayerDesign/Blueprints/PlayerCharacter.PlayerCharacter_C"))
      (`/Game/ThirdPersonBP/Blueprints2/EnemyParent_BP.UpdateHPIgnoreCD` _asenemy_parent_bp (* (`/Game/PlayerDesign/Blueprints/PlayerCharacter.ATK` _returnvalue) 0.3))
      (`SceneComponent.SetVisibility` _staticmesh false false)
      (`PrimitiveComponent.SetCollisionEnabled` _staticmesh "NoCollision"))))

(fn `UserConstructionScript`)